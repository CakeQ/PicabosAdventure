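; Auto-scrolling side camera actor that advances along world X and punishes the player for falling behind.
; Every tick it raises its speed slightly, even while stopped, and applies that speed as an unswept world offset when IsMoving is set, making scrolling frame-rate dependent.
; While moving, it calls TakeDamage on the SpriteCharacter each tick the player's capsule trails SideCamera by more than a fixed X distance.
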(event `self.ReceiveTick`
  (params (DeltaSeconds :type "Float (single-precision)"))
  (bind _camspeed (`self.CamSpeed`))
  ;[1 1 1] Move Camera
  (set `self.CamSpeed` (+ _camspeed 0.0002))
  (if (`self.IsMoving`)
    (`self.K2_AddActorWorldTransform` (`KismetMathLibrary.MakeTransform` (`KismetMathLibrary.MakeVector` _camspeed)))
    ;[1 1 1] Kill player
    (if (< (.x (`SceneComponent.K2_GetComponentLocation` (`Character.CapsuleComponent` (`GameplayStatics.GetPlayerCharacter` 0)))) (- (.x (`SceneComponent.K2_GetComponentLocation` (`self.SideCamera`))) 600.0))
      (bind _assprite_character (cast `/Game/Blueprints/Player/SpriteCharacter` (`GameplayStatics.GetPlayerCharacter` 0)))
      (`/Game/Blueprints/Player/SpriteCharacter.TakeDamage` _assprite_character))))

(fn `UserConstructionScript`)