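; Falling spike hazard that drops when its trigger box is overlapped and damages the player character on a hit.
; Any Box overlap, after a short delay, clears the inverted Fall flag, letting Tick move the Cone down a fixed step per frame without sweep, then destroys the actor.
; A custom event with a hit signature calls TakeDamage on SpriteCharacter, though its binding is not shown.
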(event `CustomEvent`
  (params (MyComp :type "PrimitiveComponent Object Reference") (Other :type "Actor Object Reference") (OtherComp :type "PrimitiveComponent Object Reference") (bSelfMoved :type Boolean :default false) (HitLocation :type "Vector Structure" :default (0.0 0.0 0.0)) (HitNormal :type "Vector Structure" :default (0.0 0.0 0.0)) (NormalImpulse :type "Vector Structure" :default (0.0 0.0 0.0)) (Hit :type "HitResult Structure (by ref)"))
  ;[1 1 1] Kill Player
  (bind _assprite_character (cast `/Game/Blueprints/Player/SpriteCharacter` Other))
  (`/Game/Blueprints/Player/SpriteCharacter.TakeDamage` _assprite_character))

(event `self.ReceiveTick`
  (params (DeltaSeconds :type "Float (single-precision)"))
  ;[1 1 1] Fall
  (if (not (`self.Fall`))
    (`SceneComponent.K2_AddRelativeLocation` (`self.Cone`) (0.0 0.0 -10.0) false false)))

(event `self.Box.OnComponentBeginOverlap`
  (params (OverlappedComponent :type "PrimitiveComponent Object Reference") (OtherActor :type "Actor Object Reference") (OtherComp :type "PrimitiveComponent Object Reference") (OtherBodyIndex :type Integer) (bFromSweep :type Boolean) (SweepResult :type "HitResult Structure (by ref)"))
  ;[1 1 1] Trigger Fall
  (`KismetSystemLibrary.Delay` 0.5)
  (set `self.Fall` false)
  (`KismetSystemLibrary.Delay` 3.0)
  (`self.K2_DestroyActor`))

(fn `UserConstructionScript`)