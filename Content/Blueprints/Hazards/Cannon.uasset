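; Cannon hazard Blueprint that repeatedly spawns Projectile actors from its Cube component.
; Tick drives a one-second Delay before each spawn, so shots repeat about every second; the trailing two-second Delay leads nowhere and does not slow firing.
; Each projectile takes the Cube's world location and scale, with its rotation yawed 180 degrees from the Cube's.
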(event `self.ReceiveTick`
  (params (DeltaSeconds :type "Float (single-precision)"))
  (`KismetSystemLibrary.Delay` 1.0)
  (`|SpawnActorFromClass` "/Game/Blueprints/Hazards/Projectile.Projectile_C" (`KismetMathLibrary.MakeTransform` (`SceneComponent.K2_GetComponentLocation` (`self.Cube`)) (`KismetMathLibrary.MakeRotator` (.roll (`SceneComponent.K2_GetComponentRotation` (`self.Cube`))) (.pitch (`SceneComponent.K2_GetComponentRotation` (`self.Cube`))) (- (.yaw (`SceneComponent.K2_GetComponentRotation` (`self.Cube`))) 180.0)) (`SceneComponent.K2_GetComponentScale` (`self.Cube`))) "Undefined" "OverrideRootScale")
  (`KismetSystemLibrary.Delay` 2.0))

(fn `UserConstructionScript`)