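; Endless side-scrolling track generator that lays pieces along X through biomes with grief-stage backdrops.
; PickTrack queues shuffled presets matching the current biome, falling back to a default Track, and randomly switches biome after a minimum length.
; Tick spawns queued pieces end to end using class-default dimensions, or, at full length, destroys those well behind the player.
; The oldest piece's biome sets the material on the player camera's background plane.
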(event `self.ReceiveBeginPlay`
  ;[1 1 1] Spawn track pieces
  (`self.ListBiomes`)
  (set `self.CurrentBiome` (`self.StartBiome`))
  (while (> (`self.TrackLength`) (`KismetArrayLibrary.Array_Length` (`self.ToSpawn`)))
    (`self.PickTrack`)
    (set `self.CameraGoFastShit` 0.0)
    (`self.SetBackground`)))

(event `self.ReceiveTick`
  (params (DeltaSeconds :type "Float (single-precision)"))
  (bind _trackpieces (`self.TrackPieces`))
  (set `self.LastBiome` (`/Game/Blueprints/Track/Track.Biome` (`|GetArrayItem` _trackpieces)))
  (`self.SetBackground`)
  (if (< (`KismetArrayLibrary.Array_Length` _trackpieces) (`self.TrackLength`))
    (`self.SpawnTrack`)
    (`self.SetBackground`)
    (else
      (for _array_element _trackpieces
        (if (> (.x (`self.K2_GetActorLocation` (`GameplayStatics.GetPlayerCharacter` 0))) (+ (+ (.x (`self.K2_GetActorLocation` _array_element)) (/ (.x (`/Game/Blueprints/Track/Track.Dimensions` _array_element)) 2.0)) 1000.0))
          (`self.K2_DestroyActor` _array_element)
          (`KismetArrayLibrary.Array_RemoveItem` _trackpieces _array_element))))))

(fn `ListBiomes`
  (bind _biometypes (`self.BiomeTypes`))
  (for _array_element (`self.TrackPresets`)
    (bind _biome (defaults `/Game/Blueprints/Sadness` _array_element))
    (if (not (`KismetArrayLibrary.Array_Contains` _biometypes _biome))
      (`KismetArrayLibrary.Array_Add` _biometypes _biome))))

(fn `PickTrack`
  (locals (FoundTrack :type Boolean) (FoundBiome :type Boolean))
  (bind _trackpresets (`self.TrackPresets`))
  (bind _foundbiome (`local.FoundBiome`))
  (bind _biometypes (`self.BiomeTypes`))
  (`KismetArrayLibrary.Array_Shuffle` _trackpresets)
  (for _array_element _trackpresets
    (if (`local.FoundTrack`)
      _
      (elif (== (defaults `/Game/Blueprints/Sadness` _array_element) (`self.CurrentBiome`))
        (`KismetArrayLibrary.Array_Add` (`self.ToSpawn`) _array_element)
        (set `self.CurrentBiomeLength` (+ (`self.CurrentBiomeLength`) 1))
        (set `local.FoundTrack` true))))
  (if (`local.FoundTrack`)
    (if (>= (`self.CurrentBiomeLength`) (`self.MinBiomeLength`))
      (if (<= (`KismetMathLibrary.RandomInteger` 100) 50)
        (`KismetArrayLibrary.Array_Shuffle` _trackpresets)
        (`KismetArrayLibrary.Array_Shuffle` _biometypes)
        (for _array_element_2 _biometypes
          (if _foundbiome
            _
            (elif (not (== _array_element_2 (`self.CurrentBiome`)))
              (set `self.CurrentBiome` _array_element_2)
              (set `self.CurrentBiomeLength` 0)
              (set `local.FoundBiome` true))))
        (if (not _foundbiome)
          (`KismetSystemLibrary.PrintString` "The generator was unable to find a new biome to use."))))
    (else
      (`KismetArrayLibrary.Array_Add` (`self.ToSpawn`) "/Game/Blueprints/Track/Default/Track.Track_C"))))

(fn `SetBackground`
  (bind _lastbiome (`self.LastBiome`))
  (bind _assprite_character (cast `/Game/Blueprints/Player/SpriteCharacter` (`GameplayStatics.GetPlayerCharacter` 0)))
  (if (== _lastbiome "A")
    (bind _plane (`/Game/Blueprints/Player/Camera.Plane` (`/Game/Blueprints/Player/SpriteCharacter.CameraRef` _assprite_character)))
    (`PrimitiveComponent.SetMaterial` _plane 0 "/Game/Materials/Track/Acceptance/Acceptance_BG.Acceptance_BG")
    (elif (== _lastbiome "B")
      (`PrimitiveComponent.SetMaterial` _plane 0 "/Game/Materials/Track/Depression/Depression_BG.Depression_BG")
      (elif (== _lastbiome "C")
        (`PrimitiveComponent.SetMaterial` _plane 0 "/Game/Materials/Track/Denial/Denial_BG.Denial_BG")
        (elif (== _lastbiome "D")
          (`PrimitiveComponent.SetMaterial` _plane 0 "/Game/Materials/Track/Bargaining/Bargaining_BG.Bargaining_BG")
          (elif (== _lastbiome "E")
            (`PrimitiveComponent.SetMaterial` _plane 0 "/Game/Materials/Track/Angry/Angry_BG.Angry_BG")))))))

(fn `SpawnTrack`
  (locals (Spawned :type Boolean))
  (bind _tospawn (`self.ToSpawn`))
  (for (_array_element _array_index) _tospawn
    (if (not (`local.Spawned`))
      (bind _returnvalue (`|SpawnActorFromClass` _array_element (`KismetMathLibrary.Conv_VectorToTransform` (`self.TrackPlacementOffset`)) "Undefined" "OverrideRootScale"))
      (`KismetArrayLibrary.Array_Add` (`self.TrackPieces`) _returnvalue)
      (set `self.TrackPlacementOffset` (`KismetMathLibrary.MakeVector` (.x (+ (`self.TrackPlacementOffset`) (`.Dimensions` (defaults `/Game/Blueprints/Sadness` _array_element))))))
      (`KismetArrayLibrary.Array_Remove` _tospawn _array_index)
      (set `local.Spawned` true)))
  (`self.PickTrack`))

(fn `UserConstructionScript`)